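; Golden fruit pickup that heals the player and advances a level quest when collected.
; Interaction requires the fruit to be unlocked in the save, then triggers player facing and regen, spawns a hit effect, flags FoundGolden on LevelManager_BP and destroys the item.
; Targeting shows a screen-space name widget and custom-depth highlight.
; Area scan toggles a screen-space marker that updates player distance in meters on Tick.
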(event EventBeginPlay
  (bind _markerwidget (Variables|Default|GetMarkerWidget))
  (bind _icon (Variables|Default|GetIcon))
  (bind _widget (Variables|Default|GetWidget))
  (bind _widget_2 (Variables|Default|GetWidget))
  (bind _returnvalue (UserInterface|GetUserWidgetObject _widget_2))
  (bind _returnvalue_2 (Transformation|GetWorldLocation _widget))
  (bind _asfood_icon_ui (Utilities|Casting|CastToFood_IconUI _returnvalue))
  ;[1 1 1] Set space to screen.
  (Class|WidgetComponent|SetWidgetSpace _widget_2 "Screen")
  (Variables|/Game/Pickups/UI/Food_IconUI.Food_IconUI_C|SetUnlockedIcon _asfood_icon_ui _icon)
  (Variables|/Game/Pickups/UI/Food_IconUI.Food_IconUI_C|SetLockedIcon _asfood_icon_ui _icon)
  (Transformation|SetWorldLocation (Variables|Default|GetMarkerWidget) (Math|Vector|MakeVector (.x _returnvalue_2) (.y _returnvalue_2) (+ (.z _returnvalue_2) 5e+01)) false false)
  (Class|WidgetComponent|SetWidgetSpace _markerwidget "Screen")
  (Default|Initialise (.AsMarker%20UI (Utilities|Casting|CastToMarker_UI (UserInterface|GetUserWidgetObject _markerwidget))) "/Game/Player/UI/AreaScan/FoodIcon.FoodIcon"))

(event EventUnlockNewItem
  ;[1 1 1] Unlock the item by setting the unlocked value in the struct to true.
  (bind _returnvalue (Actor|GetActorOfClass "/Game/Levels/LevelManager_BP.LevelManager_BP_C"))
  (Variables|/Game/Levels/LevelManager_BP.LevelManager_BP_C|SetFoundGolden? _returnvalue true)
  (Default|UpdateQuest _returnvalue 4 1))

(event EventSetAreaScanEnabled
  (params (Enabled :type Boolean))
  ;[1 1 1] Set scan area enabled for BPI
  (Rendering|SetVisibility (Variables|Default|GetMarkerWidget) Enabled false))

(event EventTick
  (params (DeltaSeconds :type Float%20%28single-precision%29))
  ;[1 1 1] Set marker distance
  (if (Rendering|IsVisible (Variables|Default|GetMarkerWidget))
    (Default|SetDistance (.AsMarker%20UI (Utilities|Casting|CastToMarker_UI (UserInterface|GetUserWidgetObject (Variables|Default|GetMarkerWidget)))) (Math|Float|Round (/ (Math|Vector|Distance(Vector) (Transformation|GetActorLocation) (Transformation|GetActorLocation (Game|GetPlayerCharacter 0))) 1e+02)))))

(event EventSetInteractTarget
  (params (NewTarget :type Boolean))
  (bind _widget (Variables|Default|GetWidget))
  ;[1 1 1] Set this as the interact target for the player.
  (Rendering|SetVisibility _widget NewTarget false)
  (Default|SetText (.AsFood%20Icon%20UI (Utilities|Casting|CastToFood_IconUI (UserInterface|GetUserWidgetObject _widget))) (Variables|Default|GetItem%20Name) true)
  (Rendering|SetRenderCustomDepth (Variables|Default|GetStaticMesh) NewTarget))

(event EventOnInteract
  (bind _returnvalue (Math|Float|MakeLiteralFloat 0.3))
  ;[1 1 1] Interface interact event. If item has been scanned before, it can be used, otherwise needs to be scanned and it will add to the diary.
  (if (.Unlocked (CallFunction|GetCondition))
    (Class|PlayerBPI|FaceItem(Message) (Game|GetPlayerCharacter 0) self 6e+01 true true 1.0)
    (Class|PlayerBPI|UpdateHealth(Message) (Game|GetPlayerCharacter 0) (Variables|Default|GetHealthAmount) true)
    (Niagara|SpawnSystematLocation "/Game/AdvancedMagicFX12/particles/Niagara/NS_ky_hit_thunder.NS_ky_hit_thunder" (Transformation|GetActorLocation) "0, 0, 0" (Math|Vector|MakeVector _returnvalue _returnvalue _returnvalue))
    (CallFunction|UnlockNewItem)
    (Actor|DestroyActor)))

(fn ConstructionScript
  (Transformation|SetWorldLocation (Variables|Default|GetWidget) (+ (Transformation|GetWorldLocation (Variables|Default|GetScan_Start)) "0.000000,0.000000,15.000000") false false))

(fn GetCondition
  (bind _savedslot (CallFunction|GetCurrentSave))
  (bind _fruit (Variables|Default|GetFruit))
  (bind _fruitsfound (Variables|/Game/SaveGame/GameSaveSlot_SG.GameSaveSlot_SG_C|GetFruitsFound _savedslot))
  (bind _value (Utilities|Map|Find _fruitsfound _fruit))
  (bind (_foodname _foodicon _itembgcolour _calories _fat _sugar _calcium _fooddescription _unlocked) (Utilities|Struct|BreakFoodItem_Struct _value))
  (return _foodname _unlocked))