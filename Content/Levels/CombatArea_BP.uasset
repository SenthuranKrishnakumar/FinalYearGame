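; Combat area actor that spawns enemies at random reachable points inside a box and activates them while the player is inside.
; Construction script sizes the box and positions side barriers with random yaw jitter, removing disabled sides.
; A screen-space marker shows player distance, toggles with area scanning, and is destroyed once death callbacks count every enemy dead.
; Player entry also unlocks a fact if LevelManager_BP's entered flag is false, but sets that flag false again.
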(event OnComponentEndOverlap(Box)
  (params (OverlappedComponent :type Primitive%20Component%20Object%20Reference) (OtherActor :type Actor%20Object%20Reference) (OtherComp :type Primitive%20Component%20Object%20Reference) (OtherBodyIndex :type Integer))
  ;[1 1 1] Disable player targetting for each enemy if the player leaves the box.
  (if (== OtherActor (Game|GetPlayerCharacter 0))
    (for _array_element (Variables|Default|GetSpawnedActors)
      (Utilities|IsValid (.AsEnemy%20Base%20Class%20Actor (Utilities|Casting|CastToEnemy_BaseClass_Actor _array_element))
        (:Is%20Valid
          (Default|SetEnemyActive (.AsEnemy%20Base%20Class%20Actor (Utilities|Casting|CastToEnemy_BaseClass_Actor _array_element)) false))))))

(event OnComponentBeginOverlap(Box)
  (params (OverlappedComponent :type Primitive%20Component%20Object%20Reference) (OtherActor :type Actor%20Object%20Reference) (OtherComp :type Primitive%20Component%20Object%20Reference) (OtherBodyIndex :type Integer) (bFromSweep :type Boolean) (SweepResult :type Hit%20Result%20Structure%20%28by%20ref%29))
  ;[1 1 1] If player enters, set each enemy to target the player and unlock fact
  (if (== OtherActor (Game|GetPlayerCharacter 0))
    (for _array_element (Variables|Default|GetSpawnedActors)
      (Utilities|IsValid (.AsEnemy%20Base%20Class%20Actor (Utilities|Casting|CastToEnemy_BaseClass_Actor _array_element))
        (:Is%20Valid
          (Default|SetEnemyActive (.AsEnemy%20Base%20Class%20Actor (Utilities|Casting|CastToEnemy_BaseClass_Actor _array_element)) true))))
    (bind _returnvalue (Actor|GetActorOfClass "/Game/Levels/LevelManager_BP.LevelManager_BP_C"))
    (if (not (Variables|/Game/Levels/LevelManager_BP.LevelManager_BP_C|GetHasEnteredCombatArea? _returnvalue))
      (Variables|/Game/Levels/LevelManager_BP.LevelManager_BP_C|SetHasEnteredCombatArea? _returnvalue false)
      (CallFunction|UnlockFact (Class|KismetSystemLibrary|MakeLiteralInteger 2) (.SavedSlotName (CallFunction|GetCurrentSave))))))

(event Custom|OnDeathCheck_Event
  ;[1 1 1] Spawn each enemy using a for loop
  (bind _result (Math|Integer|DecrementInt (Variables|Default|GetCurrentEnemies))
    (:%20%20
      (if (<= _result 0)
        (Components|DestroyComponent (Variables|Default|GetMarkerWidget))))))

(event EventBeginPlay
  (bind _markerwidget (Variables|Default|GetMarkerWidget))
  (bind _box (Variables|Default|GetBox))
  (bind _enemiestospawn (Variables|Default|GetEnemiesToSpawn))
  (bind _returnvalue (Utilities|Array|Length _enemiestospawn))
  ;[1 1 1] Initialise and marker
  (Class|WidgetComponent|SetWidgetSpace _markerwidget "Screen")
  (Default|Initialise (.AsMarker%20UI (Utilities|Casting|CastToMarker_UI (UserInterface|GetUserWidgetObject _markerwidget))) (Variables|Default|GetIcon))
  ;[1 1 1] Spawn each enemy using a for loop
  (Variables|Default|SetCurrentEnemies _returnvalue)
  (for _index (range 0 _returnvalue)
    (bind _returnvalue_2 (Game|SpawnActorfromClass (Utilities|Array|Get(acopy) _enemiestospawn _index) (Math|Transform|MakeTransform (+ (.RandomLocation (AI|Navigation|GetRandomReachablePointinRadius (Math|Random|RandomPointinBoundingBox (Transformation|GetWorldLocation _box) (Variables|/Script/Engine.BoxComponent|GetBoxExtent _box)) 5e+01 0 0)) "0.000000,0.000000,50.000000")) "AdjustIfPossibleButAlwaysSpawn" "MultiplyWithRoot" 0 0))
    (Utilities|Array|Add (Variables|Default|GetSpawnedActors) _returnvalue_2)
    (Utilities|IsValid (.AsEnemy%20Base%20Class%20Actor (Utilities|Casting|CastToEnemy_BaseClass_Actor _returnvalue_2))
      (:Is%20Valid
        (Variables|/Game/Enemies/Enemy_BaseClass_Actor.Enemy_BaseClass_Actor_C|SetEnemyRangeArea (.AsEnemy%20Base%20Class%20Actor (Utilities|Casting|CastToEnemy_BaseClass_Actor _returnvalue_2)) (Variables|Default|GetBox))
        (EventDispatchers|AssignOnDeathCheck (.AsEnemy%20Base%20Class%20Actor (Utilities|Casting|CastToEnemy_BaseClass_Actor _returnvalue_2)) (delegate Custom|OnDeathCheck_Event))))))

(event EventSetAreaScanEnabled
  (params (Enabled :type Boolean))
  (bind _markerwidget (Variables|Default|GetMarkerWidget))
  ;[1 1 1] Set visibility when area scanning
  (Utilities|IsValid _markerwidget
    (:Is%20Valid
      (Rendering|SetVisibility _markerwidget Enabled false))))

(event EventTick
  (params (DeltaSeconds :type Float%20%28single-precision%29))
  (bind _markerwidget (Variables|Default|GetMarkerWidget))
  ;[1 1 1] Initialise and marker
  (Utilities|IsValid _markerwidget
    (:Is%20Valid
      (if (Rendering|IsVisible _markerwidget)
        (Default|SetDistance (.AsMarker%20UI (Utilities|Casting|CastToMarker_UI (UserInterface|GetUserWidgetObject (Variables|Default|GetMarkerWidget)))) (Math|Float|Round (/ (Math|Vector|Distance(Vector) (Transformation|GetActorLocation) (Transformation|GetActorLocation (Game|GetPlayerCharacter 0))) 1e+02)))))))

(fn ConstructionScript
  (bind _spawnarea (Variables|Default|GetSpawnArea))
  (bind _barrierzoffset (Variables|Default|GetBarrierZOffset))
  (bind _spawnarea_2 (Variables|Default|GetSpawnArea))
  (bind _barrierzoffset_2 (Variables|Default|GetBarrierZOffset))
  (bind _returnvalue (+ (.x _spawnarea) 35.0))
  (bind _returnvalue_2 (+ (.y _spawnarea_2) 35.0))
  ;[1 1 1] Set combat area visuals
  (Components|Box|SetBoxExtent (Variables|Default|GetBox) (Variables|Default|GetSpawnArea) true)
  (Transformation|SetRelativeLocation (Variables|Default|GetLeftBarriers) (Math|Vector|MakeVector _returnvalue 0.0 _barrierzoffset) false false)
  (Transformation|SetRelativeLocation (Variables|Default|GetRightBarriers) (Math|Vector|MakeVector (* _returnvalue -1.0) 0.0 _barrierzoffset) false false)
  (Transformation|SetRelativeLocation (Variables|Default|GetFrontBarriers) (Math|Vector|MakeVector 0.0 _returnvalue_2 _barrierzoffset_2) false false)
  (Transformation|SetRelativeLocation (Variables|Default|GetBackBarriers) (Math|Vector|MakeVector 0.0 (* _returnvalue_2 -1.0) _barrierzoffset_2) false false)
  (Utilities|Array|AppendArray (Variables|Default|GetBarriers) (Components|GetChildrenComponents (Variables|Default|GetLeftBarriers) false))
  (Utilities|Array|AppendArray (Variables|Default|GetBarriers) (Components|GetChildrenComponents (Variables|Default|GetRightBarriers) false))
  (for _array_element (Variables|Default|GetBarriers)
    (Transformation|SetRelativeRotation _array_element (Math|Rotator|MakeRotator 0.0 0.0 (Math|Random|RandomFloatinRange -5.0 5.0)) false false))
  (Utilities|Array|Clear (Variables|Default|GetBarriers))
  (Utilities|Array|AppendArray (Variables|Default|GetBarriers) (Components|GetChildrenComponents (Variables|Default|GetFrontBarriers) false))
  (Utilities|Array|AppendArray (Variables|Default|GetBarriers) (Components|GetChildrenComponents (Variables|Default|GetBackBarriers) false))
  (for _array_element_2 (Variables|Default|GetBarriers)
    (Transformation|SetRelativeRotation _array_element_2 (Math|Rotator|MakeRotator 0.0 0.0 (Math|Random|RandomFloatinRange 85.0 95.0)) false false))
  (Utilities|FlowControl|Sequence
    (:then_0
      (CallFunction|DestroyBarriers (Components|GetChildrenComponents (Variables|Default|GetFrontBarriers) false)))
    (:then_1
      (CallFunction|DestroyBarriers (Components|GetChildrenComponents (Variables|Default|GetRightBarriers) false) 1))
    (:then_2
      (CallFunction|DestroyBarriers (Components|GetChildrenComponents (Variables|Default|GetBackBarriers) false) 2))
    (:then_3
      (CallFunction|DestroyBarriers (Components|GetChildrenComponents (Variables|Default|GetLeftBarriers) false) 3))))

(fn DestroyBarriers
  (params (Target :type Array%20of%20Scene%20Component%20Object%20References) (ArrayIndex :type Integer))
  (if (not (Utilities|Array|Get(acopy) (Variables|Default|GetHasBarriers) ArrayIndex))
    (for _array_element Target
      (Components|DestroyComponent _array_element))))