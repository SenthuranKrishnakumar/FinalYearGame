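; Level manager Blueprint that tracks a level's quest counters and reports whether the level's required and optional goals are met.
; BeginPlay seeds the second quest's progress from the fruits and vegetables unlocked in the current save.
; UpdateQuest increments a counter and posts it to the robot player's 2D UI.
; Helper functions compare counts against required and optional index lists, returning completion, a status enum, or remaining-count text.
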(event Custom|UpdateQuest
  (params (TargetElement :type Integer) (AddAmount :type Integer))
  (bind _levelquests (Variables|Default|GetLevelQuests))
  (bind _output (Utilities|Array|Get(acopy) _levelquests TargetElement))
  ;[1 1 1] To update a quest counter
  (Utilities|Array|SetArrayElem _levelquests TargetElement (Utilities|Struct|MakeQuest_Struct (.questdescription _output) (.updatedescription _output) (+ (.current _output) AddAmount) (.required _output)))
  (bind _returnvalue (Actor|GetActorOfClass "/Game/RobotPlayer_BP.RobotPlayer_BP_C"))
  (Default|AddUpdate (Variables|/Game/RobotPlayer_BP.RobotPlayer_BP_C|GetPlayer2DUI _returnvalue) (Utilities|Text|ToText(String) (.updatedescription _output)) (.current _output) (.required _output))
  (CallFunction|CheckCompletion))

(event EventBeginPlay
  (bind _savedslot (CallFunction|GetCurrentSave))
  (bind _levelquests (Variables|Default|GetLevelQuests))
  (bind _output (Utilities|Array|Get(acopy) _levelquests 1))
  (Utilities|Array|SetArrayElem _levelquests 1 (Utilities|Struct|MakeQuest_Struct (.questdescription _output) (.updatedescription _output) (+ (Default|FindUnlockedFruits _savedslot (Variables|Default|GetFruitsInLevel)) (Default|FindUnlockedVegetables _savedslot (Variables|Default|GetVegetablesInLevel))) (.required _output))))

(fn ConstructionScript)

(fn CheckCompletion
  (LocalVariables|SetMissingRequirements false)
  (bind _array_element (Utilities|Array|ForEachLoopwithBreak (Variables|Default|GetCompletionRequirements) :!label _label)
    (:LoopBody
      (if (!= (.current (Utilities|Array|Get(acopy) (Variables|Default|GetLevelQuests) _array_element)) (.required (Utilities|Array|Get(acopy) (Variables|Default|GetLevelQuests) _array_element)))
        (LocalVariables|SetMissingRequirements true)
        (goto _label Break)))
    (:Completed
      (return (not (LocalVariables|GetMissingRequirements))))))

(fn GetCompletionStatus
  (LocalVariables|SetMissingRequirements false)
  (bind _array_element (Utilities|Array|ForEachLoopwithBreak (Variables|Default|GetOptionalCompletionRequirements) :!label _label)
    (:LoopBody
      (if (!= (.current (Utilities|Array|Get(acopy) (Variables|Default|GetLevelQuests) _array_element)) (.required (Utilities|Array|Get(acopy) (Variables|Default|GetLevelQuests) _array_element)))
        (LocalVariables|SetMissingRequirements true)
        (goto _label Break)))
    (:Completed
      (return (select (not (LocalVariables|GetMissingRequirements)) "NewEnumerator6" "NewEnumerator7")))))

(fn GetIncomplete
  (bind _array_element (Utilities|Array|ForEachLoopwithBreak (Variables|Default|GetCompletionRequirements))
    (:LoopBody
      (if (!= (.current (Utilities|Array|Get(acopy) (Variables|Default|GetLevelQuests) _array_element)) (.required (Utilities|Array|Get(acopy) (Variables|Default|GetLevelQuests) _array_element)))
        (Utilities|Array|Add (LocalVariables|GetQuestTitle) (Utilities|String|Append (.questdescription (Utilities|Array|Get(acopy) (Variables|Default|GetLevelQuests) _array_element)) "- " (Utilities|String|ToString(Integer) (- (.required (Utilities|Array|Get(acopy) (Variables|Default|GetLevelQuests) _array_element)) (.current (Utilities|Array|Get(acopy) (Variables|Default|GetLevelQuests) _array_element)))) " Remaining!"))))
    (:Completed
      (return (LocalVariables|GetQuestTitle)))))