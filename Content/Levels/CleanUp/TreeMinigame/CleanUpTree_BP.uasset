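; Tree actor for the clean-up tree minigame that can switch between an infected and a fixed state.
; The construction script applies one mesh to both tree components and positions a point widget, which receives a reference to the tree and is shown on Activate.
; Scale and Revert play a timeline forward or backward to cross-scale the two trees, with sounds, and toggle the Infected flag.
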(event Custom|Activate
  (bind _treepointwidget (Variables|Default|GetTreePointWidget))
  ;[1 1 1] Activate by making the tree point visible and calling function in widget.
  (Rendering|SetVisibility _treepointwidget true false)
  (Default|Activate (.AsTree%20Point%20UI (Utilities|Casting|CastToTreePoint_UI (UserInterface|GetUserWidgetObject _treepointwidget)))))

(event Custom|Revert
  (bind _treescale (Variables|Default|GetTreeScale))
  ;[1 1 1] Scale the infected tree and new tree to swap between them.
  (Audio|PlaySound2D "/Game/SoundEffects/TreeShrink.TreeShrink" 1.0 1.0 0.0 0 0)
  (Variables|Default|SetInfected? true)
  (bind (_direction _value _value2) (Timeline|ScaleTree Reverse)
    (:Update
      (Transformation|SetWorldScale3D (Variables|Default|GetTree) (Math|Vector|MakeVector (Math|Float|Lerp _treescale 0.0 _value) (Math|Float|Lerp _treescale 0.0 _value) (Math|Float|Lerp _treescale 0.0 _value)))
      (Transformation|SetWorldScale3D (Variables|Default|GetFixedTree) (Math|Vector|MakeVector (Math|Float|Lerp 0.0 _treescale _value2) (Math|Float|Lerp 0.0 _treescale _value2) (Math|Float|Lerp 0.0 _treescale _value2))))))

(event Custom|Scale
  (bind _treescale (Variables|Default|GetTreeScale))
  ;[1 1 1] Scale the infected tree and new tree to swap between them.
  (Audio|PlaySound2D "/Game/SoundEffects/TreeGrow.TreeGrow" 1.0 1.0 0.0 0 0)
  (Variables|Default|SetInfected? false)
  (bind (_direction _value _value2) (Timeline|ScaleTree Play)
    (:Update
      (Transformation|SetWorldScale3D (Variables|Default|GetTree) (Math|Vector|MakeVector (Math|Float|Lerp _treescale 0.0 _value) (Math|Float|Lerp _treescale 0.0 _value) (Math|Float|Lerp _treescale 0.0 _value)))
      (Transformation|SetWorldScale3D (Variables|Default|GetFixedTree) (Math|Vector|MakeVector (Math|Float|Lerp 0.0 _treescale _value2) (Math|Float|Lerp 0.0 _treescale _value2) (Math|Float|Lerp 0.0 _treescale _value2))))))

(event EventBeginPlay
  ;[1 1 1] Find scale of tree and set references.
  (Variables|Default|SetTreeScale (.x (Transformation|GetActorScale3D)))
  (Variables|/Game/Levels/CleanUp/TreeMinigame/TreePoint_UI.TreePoint_UI_C|SetTreeRef (.AsTree%20Point%20UI (Utilities|Casting|CastToTreePoint_UI (UserInterface|GetUserWidgetObject (Variables|Default|GetTreePointWidget)))) self))

(fn ConstructionScript
  (bind _treemesh (Variables|Default|GetTreeMesh))
  (Components|StaticMesh|SetStaticMesh (Variables|Default|GetTree) _treemesh)
  (Components|StaticMesh|SetStaticMesh (Variables|Default|GetFixedTree) _treemesh)
  (Transformation|SetRelativeLocation (Variables|Default|GetTreePointWidget) (Variables|Default|GetTreePointLocation) false false))