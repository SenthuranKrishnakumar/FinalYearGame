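; Tree clean-up minigame actor, started by interacting, where infected trees are activated one by one in shuffled order.
; Interacting blends to a minigame camera with radial blur and a countdown; StartGame then advances and outlines the current tree through custom depth.
; Failure reverts healed trees using a delayed reverse-loop macro.
; Success plays a mushroom-dissolve and Niagara cutscene, returns control to the player and updates the quest.
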(event Custom|StartGame
  (bind _currenttree (Variables|Default|GetCurrentTree))
  (bind _trees (Variables|Default|GetTrees))
  (bind _output (Utilities|Array|Get(acopy) _trees _currenttree))
  (bind _asclean_up_tree_bp (Utilities|Casting|CastToCleanUpTree_BP _output))
  ;[1 1 1] Update each tree as the game progresses. Outline the current tree using post process effect.
  (if (== (Variables|Default|GetCurrentTree) (- (Utilities|Array|Length (Variables|Default|GetTrees)) 1))
    (bind _returnvalue (UserInterface|CreateWidget "/Game/Levels/CleanUp/TreeMinigame/Completion_UI.Completion_UI_C" 0 true self))
    (UserInterface|Viewport|AddtoViewport _returnvalue 0)
    (else
      (Math|Integer|IncrementInt (Variables|Default|GetCurrentTree)
        (:%20%20
          (Default|Activate _asclean_up_tree_bp)
          (bind _outactors (Actor|GetAllActorsOfClass "/Game/Levels/CleanUp/TreeMinigame/CleanUpTree_BP.CleanUpTree_BP_C"))
          (for _array_element _outactors
            (Rendering|SetRenderCustomDepth (Variables|/Game/Levels/CleanUp/TreeMinigame/CleanUpTree_BP.CleanUpTree_BP_C|GetTree _array_element) false))
          (Rendering|SetRenderCustomDepth (Variables|/Game/Levels/CleanUp/TreeMinigame/CleanUpTree_BP.CleanUpTree_BP_C|GetTree _asclean_up_tree_bp) true))))))

(event Custom|ReverseBlur
  (bind _chameleon (Variables|Default|GetChameleon))
  (bind _childactor (Variables|/Script/Engine.ChildActorComponent|GetChildActor _chameleon))
  (bind _aschameleon (Utilities|Casting|CastToChameleon _childactor))
  ;[1 1 1] When interacted, smoothly switch to the minigame camera view and hide the interaction text
  ;;[1 1 1] Add radial blur when game so more focus on infected trees
  (bind (_direction _value) (Timeline|SetBlur Reverse)
    (:Update
      (Variables|/Game/Chameleon/Chameleon.Chameleon_C|SetRadial%20Blur%20Width _aschameleon (Math|Float|Lerp 0.0 0.1 _value)))
    (:Finished
      (Variables|/Game/Chameleon/Chameleon.Chameleon_C|SetEnabled _aschameleon (Utilities|Select :Index _direction :Forward true :Backward false)))))

(event EventBeginPlay
  (bind _markerwidget (Variables|Default|GetMarkerWidget))
  (bind _trees (Variables|Default|GetTrees))
  ;[1 1 1] Initialise and marker
  (Class|WidgetComponent|SetWidgetSpace _markerwidget "Screen")
  (Default|Initialise (.AsMarker%20UI (Utilities|Casting|CastToMarker_UI (UserInterface|GetUserWidgetObject _markerwidget))) (Variables|Default|GetIcon))
  ;[1 1 1] Randomise order for minigame
  (Utilities|Array|Shuffle _trees)
  (for _array_element _trees
    (bind _asclean_up_tree_bp (Utilities|Casting|CastToCleanUpTree_BP _array_element))
    (Variables|/Game/Levels/CleanUp/TreeMinigame/TreePoint_UI.TreePoint_UI_C|SetStartedGame (.AsTree%20Point%20UI (Utilities|Casting|CastToTreePoint_UI (UserInterface|GetUserWidgetObject (Variables|/Game/Levels/CleanUp/TreeMinigame/CleanUpTree_BP.CleanUpTree_BP_C|GetTreePointWidget _asclean_up_tree_bp)))) self)))

(event EventOnFail
  ;[1 1 1] If player fails the minigame
  (Utilities|FlowControl|Sequence
    (:then_0
      ;;[1 1 1] Reverse each healed tree back to infected one by one using a custom made macro.
      (if (!= (Variables|Default|GetCurrentTree) 0)
        (for _array_element (Variables|Default|GetTrees)
          (bind _asclean_up_tree_bp (Utilities|Casting|CastToCleanUpTree_BP _array_element))
          (if (not (Variables|/Game/Levels/CleanUp/TreeMinigame/CleanUpTree_BP.CleanUpTree_BP_C|GetInfected? _asclean_up_tree_bp))
            (Utilities|Array|Add (Variables|Default|GetFixedTrees) _asclean_up_tree_bp)))
        (bind _arrayelement (Utilities|ReverseforEachLoopwithDelay (Variables|Default|GetFixedTrees) 0.1)
          (:LoopBody
            (bind _asclean_up_tree_bp_2 (Utilities|Casting|CastToCleanUpTree_BP _arrayelement))
            (Default|Revert _asclean_up_tree_bp_2))
          (:Completed
            (Variables|Default|SetCurrentTree -1)
            (Utilities|Array|Clear (Variables|Default|GetFixedTrees))))))
    (:then_1
      ;;[1 1 1] Create a failed splash screen and set the interact text back.
      (bind _returnvalue (UserInterface|CreateWidget "/Game/Levels/CleanUp/TreeMinigame/Completion_UI.Completion_UI_C" 0 false self))
      (UserInterface|Viewport|AddtoViewport _returnvalue 0)
      (Utilities|FlowControl|Delay 3.0)
      (Rendering|Components|TextRender|SetText (Variables|/Game/Levels/Interact_UI.Interact_UI_C|GetInstructionText (.AsInteract%20UI (Utilities|Casting|CastToInteract_UI (UserInterface|GetUserWidgetObject (Variables|Default|GetInteractWidget))))) "Press E to start CLEAN UP"))
    (:then_2
      ;;[1 1 1] Set all trees back to infected.
      (bind _outactors (Actor|GetAllActorsOfClass "/Game/Levels/CleanUp/TreeMinigame/CleanUpTree_BP.CleanUpTree_BP_C"))
      (for _array_element_2 _outactors
        (Variables|/Game/Levels/CleanUp/TreeMinigame/CleanUpTree_BP.CleanUpTree_BP_C|SetInfected? _array_element_2 true)))))

(event EventSetAreaScanEnabled
  (params (Enabled :type Boolean))
  (bind _markerwidget (Variables|Default|GetMarkerWidget))
  ;[1 1 1] Set visibility when area scanning
  (Utilities|IsValid _markerwidget
    (:Is%20Valid
      (Rendering|SetVisibility _markerwidget Enabled false))))

(event EventTick
  (params (DeltaSeconds :type Float%20%28single-precision%29))
  (bind _markerwidget (Variables|Default|GetMarkerWidget))
  ;[1 1 1] Initialise and marker
  (Utilities|IsValid _markerwidget
    (:Is%20Valid
      (if (Rendering|IsVisible _markerwidget)
        (Default|SetDistance (.AsMarker%20UI (Utilities|Casting|CastToMarker_UI (UserInterface|GetUserWidgetObject (Variables|Default|GetMarkerWidget)))) (Math|Float|Round (/ (Math|Vector|Distance(Vector) (Transformation|GetActorLocation) (Transformation|GetActorLocation (Game|GetPlayerCharacter 0))) 1e+02)))))))

(event EventSetInteractTarget
  (params (NewTarget :type Boolean))
  (bind _interactwidget (Variables|Default|GetInteractWidget))
  ;[1 1 1] Set this as the interact target for the player.
  (Utilities|IsValid _interactwidget
    (:Is%20Valid
      (Rendering|SetVisibility _interactwidget NewTarget false))))

(event EventOnInteract
  (bind _returnvalue (Game|GetPlayerController 0))
  (bind _chameleon (Variables|Default|GetChameleon))
  (bind _childactor (Variables|/Script/Engine.ChildActorComponent|GetChildActor _chameleon))
  (bind _aschameleon (Utilities|Casting|CastToChameleon _childactor))
  ;[1 1 1] When interacted, smoothly switch to the minigame camera view and hide the interaction text
  (Game|Player|SetViewTargetwithBlend (Game|GetPlayerController 0) (Variables|Default|GetTargetCamera) 2.5 "VTBlend_EaseInOut" 2.0 false)
  (Utilities|FlowControl|Sequence
    (:then_0
      ;;[1 1 1] Add radial blur when game so more focus on infected trees
      (Rendering|Components|TextRender|SetText (Variables|/Game/Levels/Interact_UI.Interact_UI_C|GetInstructionText (.AsInteract%20UI (Utilities|Casting|CastToInteract_UI (UserInterface|GetUserWidgetObject (Variables|Default|GetInteractWidget))))) ""))
    (:then_1
      ;;[1 1 1] Start countdown
      (Utilities|FlowControl|Delay 2.5)
      (bind _returnvalue_2 (UserInterface|CreateWidget "/Game/Levels/CleanUp/TreeMinigame/Countdown_UI.Countdown_UI_C" 0 self))
      (UserInterface|Viewport|AddtoViewport _returnvalue_2 0)
      (Input|SetInputModeGameOnly _returnvalue false)
      (Variables|/Script/Engine.PlayerController|SetbShowMouseCursor _returnvalue true)
      (Audio|PlaySound2D "/Game/SoundEffects/Countdown.Countdown" 1.0 1.0 0.0 0 0))
    (:then_2
      (Variables|/Game/Chameleon/Chameleon.Chameleon_C|SetEnabled _aschameleon true)
      (bind (_direction _value) (Timeline|SetBlur Play)
        (:Update
          (Variables|/Game/Chameleon/Chameleon.Chameleon_C|SetRadial%20Blur%20Width _aschameleon (Math|Float|Lerp 0.0 0.1 _value)))
        (:Finished
          (Variables|/Game/Chameleon/Chameleon.Chameleon_C|SetEnabled _aschameleon (Utilities|Select :Index _direction :Forward true :Backward false)))))))

(event EventOnSuccess
  (bind _returnvalue (Game|GetPlayerController 0))
  (bind _returnvalue_2 (Math|Float|MakeLiteralFloat 0.7))
  (bind _s_spotted_red_mushrooms_rdlvw_lod3_var8 (Variables|Default|GetS_Spotted_Red_Mushrooms_rdlvW_lod3_Var8))
  ;[1 1 1] If player wins the minigame
  (Audio|PlaySound2D "/Game/SoundEffects/MinigameWon.MinigameWon" 1.0 1.0 0.0 0 0)
  (Game|Player|SetViewTargetwithBlend (Game|GetPlayerController 0) (Variables|Default|GetSuccessCamera) 0.0 "VTBlend_Linear" 0.0 false)
  (Utilities|FlowControl|Delay 0.5)
  (Utilities|FlowControl|Sequence
    (:then_0
      ;;[1 1 1] Mushroom cutscene effect
      (bind _returnvalue_3 (Rendering|Material|CreateDynamicMaterialInstance _s_spotted_red_mushrooms_rdlvw_lod3_var8 0 (Rendering|Material|GetMaterial _s_spotted_red_mushrooms_rdlvw_lod3_var8 0) "None" :!class /Script/Engine.PrimitiveComponent))
      (Rendering|Material|SetMaterial _s_spotted_red_mushrooms_rdlvw_lod3_var8 0 _returnvalue_3)
      (bind _value (Timeline|ChangeMushroom Play)
        (:Update
          (Rendering|Material|SetScalarParameterValue _returnvalue_3 "Dissolve" (Math|Float|Lerp 1.0 0.0 _value) :!class /Script/Engine.MaterialInstanceDynamic)
          (Rendering|Components|Light|SetIntensity (Variables|Default|GetPointLight) (Math|Float|Lerp 5e+04 0.0 _value)))
        (:Finished
          (Components|DestroyComponent (Variables|Default|GetS_Spotted_Red_Mushrooms_rdlvW_lod3_Var5)))))
    (:then_1
      ;;[1 1 1] Particle effects
      (Niagara|SpawnSystematLocation "/Game/AdvancedMagicFX13/Particles/Niagara/NS_ky_stabShot2.NS_ky_stabShot2" (Transformation|GetActorLocation))
      (Utilities|FlowControl|Delay 1.5)
      (bind _arrayelement (Utilities|ReverseforEachLoopwithDelay (Utilities|Array|MakeArray (Variables|Default|GetPointLight) (Variables|Default|GetPointLight1) (Variables|Default|GetPointLight2) (Variables|Default|GetPointLight3)) 0.2)
        (:LoopBody
          (Niagara|SpawnSystematLocation "/Game/AdvancedMagicFX13/Particles/Niagara/NS_ky_flash1.NS_ky_flash1" (Transformation|GetWorldLocation _arrayelement) "0, 0, 0" (Math|Vector|MakeVector _returnvalue_2 _returnvalue_2 _returnvalue_2)))
        (:Completed
          (Utilities|FlowControl|Delay 1.0)
          ;;[1 1 1] Reset camera view back to player
          (bind _returnvalue_4 (Actor|GetActorOfClass "/Game/RobotPlayer_BP.RobotPlayer_BP_C"))
          (Game|Player|SetViewTargetwithBlend _returnvalue _returnvalue_4 1.5 "VTBlend_EaseInOut" 1.0 false)
          (Variables|/Script/Engine.PlayerController|SetbShowMouseCursor _returnvalue false)
          (Utilities|FlowControl|Delay 1.5)
          (Input|SetInputModeGameOnly _returnvalue true)
          (Variables|/Game/RobotPlayer_BP.RobotPlayer_BP_C|SetLockMovement _returnvalue_4 false)
          (Variables|/Game/RobotPlayer_BP.RobotPlayer_BP_C|SetIdleState _returnvalue_4 "NewEnumerator1"))))
    (:then_2
      (Components|DestroyComponent (Variables|Default|GetMarkerWidget))
      ;;[1 1 1] Update quest counter
      (bind _returnvalue_5 (Actor|GetActorOfClass "/Game/Levels/LevelManager_BP.LevelManager_BP_C"))
      (Default|UpdateQuest _returnvalue_5 3 1))))

(fn ConstructionScript)