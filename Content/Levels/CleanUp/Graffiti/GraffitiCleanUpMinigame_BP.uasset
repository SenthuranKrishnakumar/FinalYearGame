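; Interactable graffiti minigame actor where the player scrubs a decal away with a broom, then advances a quest and destroys itself.
; Interacting blends to a dedicated camera, opens Graffiti_UI and fades in radial blur.
; BroomUpdate slides the broom between two points; UpdateValue lowers the dissolve target with splash effects.
; A looping timer eases the material's Dissolve toward that target, triggering completion UI and confetti at zero.
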(event Custom|GameStarted
  (bind _returnvalue (Game|GetPlayerController 0))
  (bind _decalmat (Variables|Decal|GetDecalMat))
  (Utilities|IsValid _decalmat
    (:Is%20Valid
      (bind _returnvalue_2 (Rendering|Material|GetScalarParameterValue _decalmat "Dissolve" :!class /Script/Engine.MaterialInstanceDynamic))
      (Rendering|Material|SetScalarParameterValue _decalmat "Dissolve" (Math|Interpolation|FInterpTo _returnvalue_2 (Math|Float|Clamp(Float) (Variables|Default|GetTargetValue)) (Utilities|Time|GetWorldDeltaSeconds) 5.0) :!class /Script/Engine.MaterialInstanceDynamic)
      (if (== _returnvalue_2 0.0)
        (Utilities|FlowControl|DoOnce false
          (:Completed
            (Utilities|FlowControl|Sequence
              (:then_0
                (bind _returnvalue_3 (UserInterface|CreateWidget "/Game/Levels/CleanUp/TreeMinigame/Completion_UI.Completion_UI_C" 0 true self))
                (UserInterface|Viewport|AddtoViewport _returnvalue_3 0))
              (:then_1
                (Default|OnSuccess (Variables|Default|GetMinigameUI))
                (CallFunction|ReverseBlur)
                (Input|SetInputModeGameOnly _returnvalue false)
                (Variables|/Script/Engine.PlayerController|SetbShowMouseCursor _returnvalue false))
              (:then_2
                (Niagara|SpawnSystematLocation "/Game/Levels/CleanUp/Graffiti/Confetti_NS.Confetti_NS" (Transformation|GetActorLocation))
                (Audio|PlaySound2D "/Game/SoundEffects/MinigameWon.MinigameWon" 1.0 1.0 0.0 0 0))
              (:then_3
                (Utilities|Time|ClearandInvalidateTimerbyHandle (Variables|Default|GetGameHandle))))))))))

(event Custom|ReverseBlur
  ;[1 1 1] When interacted, switch to minigame camera and add UI.
  ;;[1 1 1] Add radial blur and scale broom
  (bind _value (Timeline|SetBlur Reverse)
    (:Update
      (Variables|/Game/Chameleon/Chameleon.Chameleon_C|SetRadial%20Blur%20Width (.AsChameleon (Utilities|Casting|CastToChameleon (Variables|/Script/Engine.ChildActorComponent|GetChildActor (Variables|Default|GetChameleon)))) (Math|Float|Lerp 0.0 0.15 _value))
      (Transformation|SetRelativeScale3D (Variables|Default|GetStaticMesh) (Math|Vector|Lerp(Vector) "0, 0, 0" (.scale (Variables|Broom|GetBroomTransform)) _value)))))

(event Custom|BroomUpdate
  (params (Value :type Float%20%28single-precision%29))
  (Transformation|SetWorldLocation (Variables|Default|GetStaticMesh) (Math|Vector|Lerp(Vector) (Transformation|GetWorldLocation (Variables|Default|GetStartPoint)) (Transformation|GetWorldLocation (Variables|Default|GetEndPoint)) Value) false false))

(event Custom|UpdateValue
  (bind _returnvalue (Math|Float|MakeLiteralFloat 0.1))
  (bind _box (Variables|Default|GetBox))
  (Variables|Default|SetTargetValue (- (Variables|Default|GetTargetValue) 0.21))
  (Audio|PlaySoundatLocation "/Game/SoundEffects/WaterSplash.WaterSplash" (Transformation|GetActorLocation) "0, 0, 0" (Math|Random|RandomFloatinRange 0.4 0.7) (Math|Random|RandomFloatinRange 0.9 1.1) 0.0 0 0 0 0)
  (for _index (range 0 6)
    (Niagara|SpawnSystematLocation "/Game/AdvancedMagicFX12/particles/Niagara/NS_ky_hit_water1.NS_ky_hit_water1" (Math|Random|RandomPointinBoundingBox (Transformation|GetWorldLocation _box) (Variables|/Script/Engine.BoxComponent|GetBoxExtent _box)) "0, 0, 0" (Math|Vector|MakeVector _returnvalue _returnvalue _returnvalue))))

(event EventBeginPlay
  (bind _markerwidget (Variables|Default|GetMarkerWidget))
  ;[1 1 1] Initialise and marker
  (Class|WidgetComponent|SetWidgetSpace _markerwidget "Screen")
  (Default|Initialise (.AsMarker%20UI (Utilities|Casting|CastToMarker_UI (UserInterface|GetUserWidgetObject _markerwidget))) (Variables|Default|GetIcon))
  (Rendering|SetVisibility (Variables|Default|GetStaticMesh) false false))

(event EventOnSuccess
  (bind _returnvalue (Game|GetPlayerController 0))
  (bind _returnvalue_2 (Actor|GetActorOfClass "/Game/RobotPlayer_BP.RobotPlayer_BP_C"))
  (Game|Player|SetViewTargetwithBlend _returnvalue _returnvalue_2 0.5 "VTBlend_Linear" 0.0 false)
  (Variables|/Script/Engine.PlayerController|SetbShowMouseCursor _returnvalue false)
  (Utilities|FlowControl|Delay 1.5)
  (Input|SetInputModeGameOnly _returnvalue true)
  (Variables|/Game/RobotPlayer_BP.RobotPlayer_BP_C|SetLockMovement _returnvalue_2 false)
  (Variables|/Game/RobotPlayer_BP.RobotPlayer_BP_C|SetIdleState _returnvalue_2 "NewEnumerator1")
  ;[1 1 1] Update quest counter
  (bind _returnvalue_3 (Actor|GetActorOfClass "/Game/Levels/LevelManager_BP.LevelManager_BP_C"))
  (Default|UpdateQuest _returnvalue_3 3 1)
  (Actor|DestroyActor))

(event EventSetAreaScanEnabled
  (params (Enabled :type Boolean))
  (bind _markerwidget (Variables|Default|GetMarkerWidget))
  ;[1 1 1] Set visibility when area scanning
  (Utilities|IsValid _markerwidget
    (:Is%20Valid
      (Rendering|SetVisibility _markerwidget Enabled false))))

(event EventTick
  (params (DeltaSeconds :type Float%20%28single-precision%29))
  (bind _markerwidget (Variables|Default|GetMarkerWidget))
  ;[1 1 1] Initialise and marker
  (Utilities|FlowControl|Sequence
    (:then_0
      (Utilities|IsValid _markerwidget
        (:Is%20Valid
          (if (Rendering|IsVisible _markerwidget)
            (Default|SetDistance (.AsMarker%20UI (Utilities|Casting|CastToMarker_UI (UserInterface|GetUserWidgetObject (Variables|Default|GetMarkerWidget)))) (Math|Float|Round (/ (Math|Vector|Distance(Vector) (Transformation|GetActorLocation) (Transformation|GetActorLocation (Game|GetPlayerCharacter 0))) 1e+02)))))))))

(event EventSetInteractTarget
  (params (NewTarget :type Boolean))
  (bind _interactwidget (Variables|Default|GetInteractWidget))
  ;[1 1 1] Set this as the interact target for the player.
  (Utilities|IsValid _interactwidget
    (:Is%20Valid
      (Rendering|SetVisibility _interactwidget NewTarget false))))

(event EventOnInteract
  (bind _returnvalue (Game|GetPlayerController 0))
  (bind _staticmesh (Variables|Default|GetStaticMesh))
  (bind _decal (Variables|Default|GetDecal))
  ;[1 1 1] When interacted, switch to minigame camera and add UI.
  (Game|Player|SetViewTargetwithBlend (Game|GetPlayerController 0) (Components|GetOwner (Variables|Default|GetCamera)) 0.5 "VTBlend_Linear" 0.0 false)
  (Utilities|FlowControl|Sequence
    (:then_0
      (Rendering|Components|TextRender|SetText (Variables|/Game/Levels/Interact_UI.Interact_UI_C|GetInstructionText (.AsInteract%20UI (Utilities|Casting|CastToInteract_UI (UserInterface|GetUserWidgetObject (Variables|Default|GetInteractWidget))))) "")
      (Transformation|SetRelativeScale3D (Variables|Default|GetStaticMesh) "0, 0, 0")
      (Rendering|SetVisibility _staticmesh true false)
      (Transformation|SetWorldLocation _staticmesh (Transformation|GetWorldLocation (Variables|Default|GetStartPoint)) false false)
      ;[1 1 1] Set dynamic material instance
      (bind _returnvalue_2 (Rendering|Material|CreateDynamicMaterialInstance _decal :!class /Script/Engine.DecalComponent))
      (Rendering|Components|Decal|SetDecalMaterial _decal _returnvalue_2)
      (Variables|Decal|SetDecalMat _returnvalue_2)
      (bind _returnvalue_3 (Utilities|Time|SetTimerbyFunctionName 0 "GameStarted" 0.001 true))
      (Variables|Default|SetGameHandle _returnvalue_3))
    (:then_1
      (bind _returnvalue_4 (UserInterface|CreateWidget "/Game/Levels/CleanUp/Graffiti/Graffiti_UI.Graffiti_UI_C" 0 self))
      (bind _output_get (Variables|Default|SetMinigameUI _returnvalue_4))
      (UserInterface|Viewport|AddtoViewport _output_get 0)
      (Input|SetInputModeUIOnly _returnvalue _output_get "DoNotLock" false)
      (Variables|/Script/Engine.PlayerController|SetbShowMouseCursor _returnvalue true))
    (:then_2
      ;;[1 1 1] Add radial blur and scale broom
      (bind _value (Timeline|SetBlur Play)
        (:Update
          (Variables|/Game/Chameleon/Chameleon.Chameleon_C|SetRadial%20Blur%20Width (.AsChameleon (Utilities|Casting|CastToChameleon (Variables|/Script/Engine.ChildActorComponent|GetChildActor (Variables|Default|GetChameleon)))) (Math|Float|Lerp 0.0 0.15 _value))
          (Transformation|SetRelativeScale3D (Variables|Default|GetStaticMesh) (Math|Vector|Lerp(Vector) "0, 0, 0" (.scale (Variables|Broom|GetBroomTransform)) _value)))))))

(fn ConstructionScript
  (bind _decal (Variables|Default|GetDecal))
  (Rendering|Components|Decal|SetDecalMaterial _decal (Variables|Decal|GetDecalMaterial))
  (Transformation|SetWorldScale3D _decal (Variables|Decal|GetDecalSize))
  (Transformation|SetRelativeRotation (Variables|Default|GetBox) (Variables|Decal|GetDecalRotation) false false)
  (Components|Box|SetBoxExtent (Variables|Default|GetBox) (Variables|Box|GetBoxExtent) true)
  (Transformation|SetRelativeTransform (Variables|Default|GetCamera) (Variables|Camera|GetCameraTransform) false false)
  (Transformation|SetRelativeTransform (Variables|Default|GetStaticMesh) (Variables|Broom|GetBroomTransform) false false)
  (Transformation|SetRelativeLocation (Variables|Default|GetStartPoint) (Variables|Broom|GetStartLocation) false false)
  (Transformation|SetRelativeLocation (Variables|Default|GetEndPoint) (Variables|Broom|GetEndLocation) false false)
  (Transformation|SetWorldLocation (Variables|Default|GetStaticMesh) (Transformation|GetWorldLocation (select (Variables|Default|GetDebugEnd?) (Variables|Default|GetEndPoint) (Variables|Default|GetStartPoint))) false false))