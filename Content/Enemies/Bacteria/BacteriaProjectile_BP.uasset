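; Projectile for the Bacteria enemy that damages what it hits and expires after a fixed lifespan.
; Sphere overlaps with WorldStatic or Pawn objects, excluding its spawner, send a randomised health update to the other actor, then destroy the projectile with an impact effect and sound.
; The selected colour tints both the projectile and impact Niagara effects, while start and impact sounds vary randomly in volume and pitch.
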(event OnComponentBeginOverlap(Sphere)
  (params (OverlappedComponent :type Primitive%20Component%20Object%20Reference) (OtherActor :type Actor%20Object%20Reference) (OtherComp :type Primitive%20Component%20Object%20Reference) (OtherBodyIndex :type Integer) (bFromSweep :type Boolean) (SweepResult :type Hit%20Result%20Structure%20%28by%20ref%29))
  (bind _returnvalue (Collision|GetCollisionObjectType OtherComp))
  ;[1 1 1] On hit detected
  (if (and (or (Utilities|Enum|Equal(Enum) _returnvalue "ECC_WorldStatic") (Utilities|Enum|Equal(Enum) _returnvalue "ECC_Pawn")) (!= OtherActor (Variables|Default|GetSpawnedBy)))
    (bind _returnvalue_2 (Niagara|SpawnSystematLocation "/Game/AdvancedMagicFX12/particles/Niagara/NS_BacteriaProjectileHit.NS_BacteriaProjectileHit" (Transformation|GetActorLocation)))
    (Class|PlayerBPI|UpdateHealth(Message) OtherActor (Math|Random|RandomFloatinRange 1e+01 15.0) false)
    (Niagara|SetNiagaraVariable(LinearColor) _returnvalue_2 "Colour" (Variables|Default|GetSelectedColour))
    (Audio|PlaySoundatLocation "/Game/SoundEffects/ProjectileImpact.ProjectileImpact" (Transformation|GetActorLocation) "0, 0, 0" (Math|Random|RandomFloatinRange 0.4 0.7) (Math|Random|RandomFloatinRange 0.9 1.1) 0.0 0 0 0 0)
    (Actor|DestroyActor)))

(event EventBeginPlay
  ;[1 1 1] Auto destroy if nothing hit
  (Actor|SetLifeSpan 2e+01)
  (Audio|PlaySoundatLocation "/Game/SoundEffects/ProjectileStart.ProjectileStart" (Transformation|GetActorLocation) "0, 0, 0" (Math|Random|RandomFloatinRange 0.4 0.7) (Math|Random|RandomFloatinRange 0.9 1.1) 0.0 0 0 0 0))

(fn ConstructionScript
  (AddComponent|AddSplineMeshComponent false)
  (Niagara|SetNiagaraVariable(LinearColor) (Variables|Default|GetNiagara) "Colour" (Variables|Default|GetSelectedColour)))