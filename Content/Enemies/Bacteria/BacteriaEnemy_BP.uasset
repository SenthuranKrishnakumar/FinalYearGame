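; Bacteria enemy that faces the player in range and randomly picks a melee or ranged attack.
; Melee moves to the player, spawns tentacle-tip particles and damages sphere-trace hits, while ranged fires a projectile at the player.
; BeginPlay picks a random colour shared by materials, death particle, attack effects and projectile, and starts blink morphs and ambient sounds.
; Hits play a hurt montage; death animates and scales the mesh before destroying the actor.
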(event EventBeginPlay
  (bind _colours (Variables|Default|GetColours))
  ;[1 1 1] Set random colour.
  (Utilities|FlowControl|Sequence
    (:then_0
      (|CallParentFunction))
    (:then_1
      (Variables|Default|SetSelectedColour (Utilities|Array|Get(acopy) _colours (Math|Random|RandomIntegerinRange 0 (- (Utilities|Array|Length _colours) 1))))
      (CallFunction|SetParameter 0 "Albedo Tint" (Variables|Default|GetSelectedColour))
      (CallFunction|SetParameter 1 "Albedo Tint" (Math|Color|Lerp(LinearColor) :A (Variables|Default|GetSelectedColour) :Alpha 0.9))
      (CallFunction|SetParameter 5 "Colour" (Math|Color|Lerp(LinearColor) :A (Variables|Default|GetSelectedColour) :Alpha 0.9))
      (Niagara|SetNiagaraVariable(LinearColor) (Variables|Default|GetDeath_Particle) "Colour" (Variables|Default|GetSelectedColour)))
    (:then_2
      ;;[1 1 1] Blink with random intervals. Modify morph target to create blinking.
      (bind _value (Timeline|Blink PlayFromStart)
        (:Update
          (Components|SkeletalMesh|SetMorphTarget (Variables|Character|GetMesh) "Blink" (Math|Float|Lerp 0.0 1.2 _value) true)
          (Utilities|FlowControl|Delay (Math|Random|RandomFloatinRange 3.0 4.0))
          (Timeline|Blink PlayFromStart))))
    (:then_3
      (Utilities|FlowControl|RetriggerableDelay (Math|Random|RandomFloatinRange 8.0 12.0) :!label _label)
      (if (Math|Random|RandomBool)
        (Audio|PlaySoundatLocation "/Game/SoundEffects/MonsterAmbient_Cue.MonsterAmbient_Cue" (Transformation|GetActorLocation) "0, 0, 0" (Math|Random|RandomFloatinRange 0.4 0.7) (Math|Random|RandomFloatinRange 0.9 1.1) 0.0 0 0 0 0)
        (goto _label)))))

(event EventOnDeath
  ;[1 1 1] Play animation and scale enemy on death.
  (Utilities|FlowControl|Sequence
    (:then_0
      (Components|Animation|PlayAnimation (Variables|Character|GetMesh) "/Game/Enemies/Bacteria/Animations/Death.Death" false)
      (bind _value (Timeline|Fade PlayFromStart)
        (:Update
          (Transformation|SetRelativeScale3D (Variables|Character|GetMesh) (Math|Vector|Lerp(Vector) "0, 0, 0" "0.400000,0.400000,0.400000" _value)))
        (:Finished
          (Actor|DestroyActor))))
    (:then_1
      (Audio|PlaySoundatLocation "/Game/SoundEffects/MonsterDeath2.MonsterDeath2" (Transformation|GetActorLocation) "0, 0, 0" (Math|Random|RandomFloatinRange 0.4 0.7) (Math|Random|RandomFloatinRange 0.9 1.1) 0.0 0 0 0 0))))

(event EventAIBehaviour
  (bind _returnvalue (Math|Float|MakeLiteralFloat 0.8))
  (bind _mesh (Variables|Character|GetMesh))
  (bind _returnvalue_2 (Transformation|GetWorldLocation _mesh))
  ;[1 1 1] Melee attack.Spawn particle at each tentacle. Use sphere trace to detect damageable objects in range.
  (bind _output_get (Variables|Default|SetAttackType (Utilities|Enum|ByteToEnumBacteriaAttack_Enum (Math|Conversions|ToByte(Integer) (Math|Random|RandomIntegerinRange 0 1)))))
  (switch Utilities|FlowControl|Switch|SwitchonBacteriaAttack_Enum _output_get
    (:NewEnumerator1
      (AI|AIMoveTo self (Transformation|GetActorLocation (Game|Player|GetPlayerPawn 0)) 0 2e+01 true
        (:OnSuccess
          _)
        (:OnFail
          _))
      (if (Collision|IsOverlappingActor (Variables|Default|GetSphere) (Game|GetPlayerCharacter 0) :!class /Script/Engine.PrimitiveComponent)
        (Utilities|FlowControl|DoOnce false :!label _label
          (:Completed
            (Utilities|FlowControl|Sequence
              (:then_0
                (for _array_element (Utilities|Array|MakeArray "Bone_end" "Bone_001_end" "Bone_002_end" "Bone_003_end" "Bone_004_end" "Bone_005_end")
                  (bind _returnvalue_3 (Niagara|SpawnSystemAttached "/Game/AdvancedMagicFX12/particles/Niagara/NS_BacteriaAttack.NS_BacteriaAttack" (Variables|Character|GetMesh) _array_element "0, 0, 0" "0, 0, 0" "KeepRelativeOffset" true false))
                  (Transformation|SetWorldScale3D _returnvalue_3 (Math|Vector|MakeVector _returnvalue _returnvalue _returnvalue))
                  (Niagara|SetNiagaraVariable(LinearColor) _returnvalue_3 "Colour" (Variables|Default|GetSelectedColour))
                  (Components|Activation|Activate _returnvalue_3 false)
                  (Audio|PlaySoundatLocation "/Game/SoundEffects/BacteriaMelee.BacteriaMelee" (Transformation|GetActorLocation) "0, 0, 0" (Math|Random|RandomFloatinRange 0.4 0.7) (Math|Random|RandomFloatinRange 0.9 1.1) 0.0 0 0 0 0)))
              (:then_1
                (bind _outhits (Collision|MultiSphereTraceByChannel _returnvalue_2 _returnvalue_2 1e+02 "TraceTypeQuery1" false (Utilities|Array|MakeArray self) "None"))
                (for _array_element_2 _outhits
                  (Class|PlayerBPI|UpdateHealth(Message) (.HitActor (Collision|BreakHitResult _array_element_2)) (Math|Random|RandomFloatinRange 15.0 2e+01) false)))
              (:then_2
                (Utilities|FlowControl|Delay 0.2)
                (goto _label Reset)))))))
    (:NewEnumerator8
      ;[1 1 1] Spawn projectile. Find rotation using find look at rotation to player.
      (Variables|Default|SetInterp%20Speed 15.0)
      (Game|SpawnActorfromClass "/Game/Enemies/Bacteria/BacteriaProjectile_BP.BacteriaProjectile_BP_C" (Math|Transform|MakeTransform (Transformation|GetWorldLocation (Variables|Character|GetMesh)) (Math|Rotator|FindLookatRotation (Transformation|GetActorLocation) (Transformation|GetActorLocation (Game|GetPlayerCharacter 0)))) "Undefined" "MultiplyWithRoot" 0 self (Variables|Default|GetSelectedColour) 0))))

(event EventTick
  (params (DeltaSeconds :type Float%20%28single-precision%29))
  ;[1 1 1] For smooth rotation when facing enemy.
  (if (Variables|Default|GetPlayerInRange?)
    (Transformation|SetActorRotation (Math|Interpolation|RInterpTo (Transformation|GetActorRotation) (Math|Rotator|FindLookatRotation (Transformation|GetActorLocation) (Transformation|GetActorLocation (Game|GetPlayerCharacter 0))) (Utilities|Time|GetWorldDeltaSeconds) (Variables|Default|GetInterp%20Speed)))))

(fn ConstructionScript
  (|CallParentFunction))

(fn SetParameter
  (params (ElementIndex :type Integer) (ParameterName :type Name) (Value :type Linear%20Color%20Structure))
  (bind _mesh (Variables|Character|GetMesh))
  (bind _returnvalue (Rendering|Material|CreateDynamicMaterialInstance _mesh ElementIndex (Rendering|Material|GetMaterial _mesh ElementIndex) "None" :!class /Script/Engine.PrimitiveComponent))
  (Rendering|Material|SetVectorParameterValue _returnvalue ParameterName Value :!class /Script/Engine.MaterialInstanceDynamic))

(fn SecondaryHitReaction
  (Animation|Montage|MontagePlay (Components|SkeletalMesh|GetAnimInstance (Variables|Character|GetMesh)) "/Game/Enemies/Bacteria/Animations/Hurt_Montage.Hurt_Montage" 1.0 "MontageLength" 0.0 true)
  (Audio|PlaySoundatLocation "/Game/SoundEffects/HitImpact.HitImpact" (Transformation|GetActorLocation) "0, 0, 0" (Math|Random|RandomFloatinRange 0.4 0.7) (Math|Random|RandomFloatinRange 0.9 1.1) 0.0 0 0 0 0))