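; Companion wolf character that follows the player, roams nearby, and sits or resumes on interaction.
; BeginPlay applies saved customisation textures to mesh materials through dynamic instances.
; Tick sprints it to the player's follow point when out of range unless sitting, while a CurrentState-driven loop scouts random reachable points with randomised idle waits, lying down on longer ones.
; Interacting within sphere overlap toggles sitting, and a seated, out-of-range wolf chases the player.
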(event Custom|AI_CheckState
  (bind _idlemin (Variables|Default|GetIdleMin))
  (bind _idlemax (Variables|Default|GetIdleMax))
  ;[1 1 1] If in player range, walk around near them.
  (if (and (< (Transformation|GetDistanceTo (Game|Player|GetPlayerPawn 0) self) (Variables|Default|GetMinDistanceToPlayer)) (Math|Boolean|ORBoolean (Utilities|Enum|Equal(Enum) (Variables|Default|GetCurrentState) "NewEnumerator0") (Utilities|Enum|Equal(Enum) (Variables|Default|GetCurrentState) "NewEnumerator1") (Utilities|Enum|Equal(Enum) (Variables|Default|GetCurrentState) "NewEnumerator6")))
    (Variables|Default|SetCurrentState "NewEnumerator1")
    (AI|AIMoveTo self (.RandomLocation (AI|Navigation|GetRandomReachablePointinRadius (Transformation|GetActorLocation (Game|Player|GetPlayerPawn 0)) (Variables|Default|GetScoutRadius) 0 0)) 0 1e+02 true
      (:OnSuccess
        _)
      (:OnFail
        _))
    (if (Utilities|Enum|NotEqual(Enum) (Variables|Default|GetCurrentState) "NewEnumerator3")
      (bind _output_get (Variables|Default|SetIdleWaitTime (Math|Random|RandomFloatinRange _idlemin _idlemax)))
      (Utilities|FlowControl|Sequence
        (:then_0
          (Utilities|FlowControl|RetriggerableDelay _output_get)
          (CallFunction|AICheckState))
        (:then_1
          (if (> _output_get (/ (+ _idlemin _idlemax) 2.0))
            (Variables|Default|SetCurrentState "NewEnumerator6")))))))

(event Custom|WolfInteractToggle
  (bind _charactermovement (Variables|Character|GetCharacterMovement))
  ;[1 1 1] Sit, chase or stand based on current state of the wolf.
  (switch Utilities|FlowControl|Switch|SwitchonWolfState_Enum (Variables|Default|GetCurrentState)
    (:NewEnumerator0
      (if (Variables|Default|GetIsInPlayerRange) :!label _label
        (Variables|/Script/Engine.CharacterMovementComponent|SetMaxWalkSpeed _charactermovement 0.0)
        (Components|Movement|StopMovementImmediately _charactermovement)
        (Class|NavMovementComponent|StopActiveMovement _charactermovement)
        (Variables|Default|SetCurrentState "NewEnumerator3")))
    (:NewEnumerator3
      (if (Variables|Default|GetIsInPlayerRange)
        (Variables|/Script/Engine.CharacterMovementComponent|SetMaxWalkSpeed (Variables|Character|GetCharacterMovement) (Variables|Default|GetWalkSpeed))
        (Variables|Default|SetCurrentState "NewEnumerator0")
        (CallFunction|AICheckState)
        (else
          (Variables|Default|SetCurrentState "NewEnumerator5")
          (Variables|/Script/Engine.CharacterMovementComponent|SetMaxWalkSpeed (Variables|Character|GetCharacterMovement) 6e+02)
          (AI|AIMoveTo self (.RandomLocation (AI|Navigation|GetRandomReachablePointinRadius (Transformation|GetWorldLocation (Variables|/Game/RobotPlayer_BP.RobotPlayer_BP_C|GetWolfFollowPoint (.AsRobot%20Player%20BP (Utilities|Casting|CastToRobotPlayer_BP (Game|Player|GetPlayerPawn 0))))) 15.0 0 0)) 0 5.0 true
            (:OnSuccess
              (Variables|Default|SetCurrentState "NewEnumerator0"))))))
    (:NewEnumerator1
      (goto _label))
    (:NewEnumerator4
      (goto _label))
    (:NewEnumerator5
      (goto _label))
    (:NewEnumerator6
      (goto _label))))

(event EventBeginPlay
  (bind _savedslot (CallFunction|GetCurrentSave))
  (bind _mesh (Variables|Character|GetMesh))
  (bind _wolfcostumisation_textures (Variables|/Game/SaveGame/GameSaveSlot_SG.GameSaveSlot_SG_C|GetWolfCostumisation_Textures _savedslot))
  ;[1 1 1] Set wolf skin.
  (Utilities|FlowControl|Sequence
    (:then_0
      (bind _keys (Utilities|Map|Keys _wolfcostumisation_textures))
      (for (_array_element _array_index) _keys
        (bind _values (Utilities|Map|Values _wolfcostumisation_textures))
        (bind _returnvalue (Rendering|Material|CreateDynamicMaterialInstance (Variables|Character|GetMesh) (Rendering|Material|GetMaterialIndex _mesh _array_element) (Rendering|Material|GetMaterial _mesh (Rendering|Material|GetMaterialIndex _mesh _array_element)) "None" :!class /Script/Engine.PrimitiveComponent))
        (Rendering|Material|SetTextureParameterValue _returnvalue "Diffuse" (Utilities|Array|Get(acopy) _values _array_index))))
    (:then_1
      (CallFunction|AICheckState))))

(event EventTick
  (params (DeltaSeconds :type Float%20%28single-precision%29))
  ;[1 1 1] If player is not in range of wolf, follow.
  (Utilities|FlowControl|Sequence
    (:then_0
      (if (not (< (Transformation|GetDistanceTo (Game|Player|GetPlayerPawn 0) self) (Variables|Default|GetMinDistanceToPlayer)))
        (if (Utilities|Enum|NotEqual(Enum) (Variables|Default|GetCurrentState) "NewEnumerator3")
          (Variables|/Script/Engine.CharacterMovementComponent|SetMaxWalkSpeed (Variables|Character|GetCharacterMovement) (Variables|Default|GetSprintSpeed))
          (Variables|Default|SetCurrentState "NewEnumerator4")
          (AI|AIMoveTo self (.RandomLocation (AI|Navigation|GetRandomReachablePointinRadius (Transformation|GetWorldLocation (Variables|/Game/RobotPlayer_BP.RobotPlayer_BP_C|GetWolfFollowPoint (.AsRobot%20Player%20BP (Utilities|Casting|CastToRobotPlayer_BP (Game|Player|GetPlayerPawn 0))))) 15.0 0 0)) 0 5.0 true
            (:OnSuccess
              (Variables|/Script/Engine.CharacterMovementComponent|SetMaxWalkSpeed (Variables|Character|GetCharacterMovement) (Math|Float|SelectFloat 175.0 (Variables|Default|GetSprintSpeed) (< (Transformation|GetDistanceTo (Game|Player|GetPlayerPawn 0) self) (Variables|Default|GetMinDistanceToPlayer))))
              (Variables|Default|SetCurrentState "NewEnumerator0"))
            (:OnFail
              _))
          (CallFunction|AICheckState))))
    (:then_1
      (Variables|Default|SetIsInPlayerRange (Collision|IsOverlappingActor (Variables|Default|GetSphere) (Game|Player|GetPlayerPawn 0) :!class /Script/Engine.PrimitiveComponent)))))

(fn ConstructionScript)